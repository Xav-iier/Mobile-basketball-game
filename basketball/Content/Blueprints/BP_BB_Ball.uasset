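; BP_BB_Ball is a ball actor that is launched as a projectile along a given direction.
; Launch scales the normalized direction by Power, adds a small upward Z bias, then multiplies by Power again, so directional speed grows with Power squared.
; It passes the result to the Projectile component as a local-space velocity and activates it; the event graph and construction script are empty.
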(fn `Launch`
  (params (DIR :type "Vector Structure") (power :type "Float (double-precision)"))
  (`ProjectileMovementComponent.SetVelocityInLocalSpace` (`self.Projectile`) (* (`KismetMathLibrary.MakeVector` (.x (* (`KismetMathLibrary.Normal` DIR) power)) (.y (* (`KismetMathLibrary.Normal` DIR) power)) (+ (.z (* (`KismetMathLibrary.Normal` DIR) power)) 0.25)) (`self.Power`)))
  (`ActorComponent.Activate` (`self.Projectile`) false)
  (return))

(fn `UserConstructionScript`)